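; BP_PL_Pottery_Testmod is a test-mod pottery object that exercises a server RPC from its interaction menu.
; It extends the parent's radial menu with an "RPC Test" entry bound to a click event.
; Clicking shows a notification, then passes the object to ServerRPCTestWithBaseItem on the first player character's BP_AC_Testmod component, routing the RPC through the player rather than the object.
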(event `self.InteractableMenu`
  (params (RadialMenu :type "RadialMenu Object Reference") (HitIndex :type Integer))
  (`parent.InteractableMenu` RadialMenu HitIndex)
  (bind _asw_radial_menu (cast `/Game/UI/Framework/W_RadialMenu` RadialMenu))
  (bind _returnvalue (`RadialMenu.AddItem` _asw_radial_menu "RPC Test" "" "/Game/UI/Textures/GUIs/MainRadialMenu/T_MainRadialMenuIconLootAll.T_MainRadialMenuIconLootAll" "None" -1))
  (add `RadialMenuEntry.SignalClicked` _returnvalue (delegate `Event Clicked`)))

(event `Event Clicked`
  (params (menuEntry :type "RadialMenuEntry Object Reference"))
  (message `/Game/Characters/HUDNotification_Interface.NotificationText` (`GameplayStatics.GetPlayerController` 0) "RPC Test" false)
  (`/Game/Mods/Testmod01/BP_AC_Testmod.Server RPC Test With BaseItem` (`self.GetComponentByClass` (`GameplayStatics.GetPlayerCharacter` 0) "/Game/Mods/Testmod01/BP_AC_Testmod.BP_AC_Testmod_C") self))

(fn `UserConstructionScript`
  (`parent.UserConstructionScript`))